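; BP_BoxActor is a box actor in the FPS content with a health value shown through a WBP_Health widget component.
; On BeginPlay it casts the component's widget to WBP_Health, caches it and gives it a reference back to the box.
; The UpdateHealth event copies BoxHealth into the widget when that cached reference is valid.
; The graph itself contains no damage logic and does not call UpdateHealth.
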(event `self.ReceiveBeginPlay`
  (bind _aswbp_health (cast `/Game/_FPS/HUD/Widgets/WBP_Health` (`WidgetComponent.GetUserWidgetObject` (`self.HealthWidget`))))
  (bind _output_get (set `self.As WBP Health` _aswbp_health))
  (set `/Game/_FPS/HUD/Widgets/WBP_Health.BoxActorBP` self _output_get))

(event `self.UpdateHealth`
  (`/Engine/EditorBlueprintResources/StandardMacros.IsValid` (`self.As WBP Health`)
    (:`Is Valid`
      (set `/Game/_FPS/HUD/Widgets/WBP_Health.BoxHealthWidget` (`self.BoxHealth`) (`self.As WBP Health`)))))

(fn `UserConstructionScript`)